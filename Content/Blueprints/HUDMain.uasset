(event `self.ReceiveDrawHUD`
  (params (SizeX :type Integer) (SizeY :type Integer))
  (bind _returnvalue (`KismetMathLibrary.Conv_IntToDouble` SizeX))
  (bind _returnvalue_2 (`KismetMathLibrary.Conv_IntToDouble` SizeY))
  (bind (_outwidth _outheight) (`self.GetTextSize` "You Lose" "/Game/Blueprints/SegueUI.SegueUI" 1.0))
  (bind (_outwidth_2 _outheight_2) (`self.GetTextSize` "Speed Boosted!" "/Game/Blueprints/SegueUI.SegueUI"))
  (bind (_outwidth_3 _outheight_3) (`self.GetTextSize` "You Win" "/Game/Blueprints/SegueUI.SegueUI"))
  (`|ExecutionSequence`
    (:`then_0`
      ;[1 1 1] Check if isDead
      (if (`/Game/Blueprints/MyCharacter.isDead` (stale `self.ReceiveBeginPlay` _asmycharacter_c))
        (`self.DrawText` "You Lose" (struct :`R` 0.751895 :`G` 0.751895 :`B` 0.751895 :`A` 1.0) (/ (- _returnvalue _outwidth) 2.0) (/ (- _returnvalue_2 _outheight) 2.0) "/Game/Blueprints/SegueUI.SegueUI")
        (elif (not (`/Game/Blueprints/MyCharacter.caughtRunner` (stale `self.ReceiveBeginPlay` _asmycharacter_c)))
          ;[1 1 1] Coins
          (`self.DrawText` "Coins: 0" (struct :`R` 0.751895 :`G` 0.751895 :`B` 0.751895 :`A` 1.0) 0.0 0.0 "/Game/Blueprints/SegueUI.SegueUI" 1.0))))
    (:`then_1`
      ;[1 1 1] Check if caughtRunner
      (if (`/Game/Blueprints/MyCharacter.caughtRunner` (stale `self.ReceiveBeginPlay` _asmycharacter_c))
        (`self.DrawText` "You Win" (struct :`R` 0.751895 :`G` 0.751895 :`B` 0.751895 :`A` 1.0) (/ (- _returnvalue _outwidth_3) 2.0) (/ (- _returnvalue_2 _outheight_3) 2.0) "/Game/Blueprints/SegueUI.SegueUI")))
    (:`then_2`
      ;[1 1 1] Check if isBoosted
      (if (`/Game/Blueprints/MyCharacter.isBoosted` (stale `self.ReceiveBeginPlay` _asmycharacter_c))
        (`self.DrawText` "Speed Boosted!" (struct :`R` 0.751895 :`G` 0.751895 :`B` 0.751895 :`A` 1.0) (/ (- _returnvalue _outwidth_2) 2.0) (/ (- _returnvalue_2 _outheight_2) 2.0) "/Game/Blueprints/SegueUI.SegueUI")
        (`KismetSystemLibrary.Delay` 2.0)
        (set `/Game/Blueprints/MyCharacter.isBoosted` false (stale `self.ReceiveBeginPlay` _asmycharacter_c))))))

(event `self.ReceiveBeginPlay`
  (bind _asmycharacter_c (cast `/Game/Blueprints/MyCharacter` (`GameplayStatics.GetPlayerCharacter` 0))))

(fn `UserConstructionScript`)