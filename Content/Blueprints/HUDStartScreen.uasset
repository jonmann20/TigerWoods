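; HUD Blueprint for the start screen, showing the game title "Tiger Woods" and a touch-to-start prompt.
; On each DrawHUD it draws both strings in light grey Segue UI text, measuring each with GetTextSize to center it.
; The larger title is centered horizontally at the top edge, while the prompt is centered both horizontally and vertically.
; It only draws text and handles no input.
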(event `self.ReceiveDrawHUD`
  (params (SizeX :type Integer) (SizeY :type Integer))
  (bind (_outwidth _outheight) (`self.GetTextSize` "Touch screen to start" "/Game/Blueprints/SegueUI.SegueUI"))
  (bind _returnvalue (`KismetMathLibrary.Conv_IntToDouble` SizeX))
  (`|ExecutionSequence`
    (:`then_0`
      (`self.DrawText` "Tiger Woods" (struct :`R` 0.751895 :`G` 0.751895 :`B` 0.751895 :`A` 1.0) (/ (- _returnvalue (`self.GetTextSize` "Tiger Woods" "/Game/Blueprints/SegueUI.SegueUI" 1.5)) 2.0) 0.0 "/Game/Blueprints/SegueUI.SegueUI" 1.5))
    (:`then_1`
      (`self.DrawText` "Touch screen to start" (struct :`R` 0.751895 :`G` 0.751895 :`B` 0.751895 :`A` 1.0) (/ (- _returnvalue _outwidth) 2.0) (/ (- (`KismetMathLibrary.Conv_IntToDouble` SizeY) _outheight) 2.0) "/Game/Blueprints/SegueUI.SegueUI"))))

(fn `UserConstructionScript`)